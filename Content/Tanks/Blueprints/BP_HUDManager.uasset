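; BP_HUDManager manages the tank game's HUD widgets, with all display logic skipped when IsMenuOnly is set.
; It adds the player health bar on BeginPlay, and pauses the game with the game-over menu when DestroyingBindActor fires.
; CallTurretList uses a FlipFlop to alternately show and hide the turret list.
; Hiding binds to the ShowHide animation's finish to remove the widget from the viewport.
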(event Custom|Event%20Call%20Turret%20List
  (if (not (Variables|Default|GetbIsMenuOnly))
    (Utilities|FlowControl|FlipFlop
      (:A
        (bind _returnvalue (Class|HUDManager|AddWidgettoViewport "TurretList"))
        (bind _output_get (Variables|Default|SetTurretListWidget _returnvalue))
        (bind _aswbp_turret_list (Utilities|Casting|CastToWBP_TurretList _output_get))
        (Default|EventShow _aswbp_turret_list))
      (:B
        (bind _turretlistwidget (Variables|Default|GetTurretListWidget)
          (:then
            (bind _aswbp_turret_list_2 (Utilities|Casting|CastToWBP_TurretList _turretlistwidget))
            (Default|EventHide _aswbp_turret_list_2)
            (Class|UserWidget|BindtoAnimationFinished _aswbp_turret_list_2 (Variables|/Game/Tanks/UI/WBP_TurretList.WBP_TurretList_C|GetShowHide _aswbp_turret_list_2) (delegate Custom|Event%20Remove%20Widget)))
          (:else))))))

(event Custom|Event%20Remove%20Widget
  (bind _turretlistwidget (Variables|Default|GetTurretListWidget)
    (:then
      (Class|HUDManager|RemoveWidgetfromViewport _turretlistwidget))
    (:else)))

(event EventBeginPlay
  (if (not (Variables|Default|GetbIsMenuOnly))
    (Class|HUDManager|AddWidgettoViewport "PlayerHealthBar")))

(event EventDestroyingBindActor
  (if (not (Variables|Default|GetbIsMenuOnly))
    (Game|SetGamePaused true)
    (Class|HUDManager|AddWidgettoViewport "GameOverMenu")))

(fn ConstructionScript)